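; BP_Rod is a VR-pickable rod that mounts onto the Aquilos.
; When its attach box overlaps the Aquilos cap with both fixing knobs unlocked, it snaps to the S_Rod socket and releases the grasp.
; Tick disables pickability and collision while it is mounted and either knob is locked.
; Tick also resets AttachTo to Else when a motion controller takes it from the Aquilos or Work Station.
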(event OnComponentBeginOverlap(Box_AttachToAquilos)
  (params (OverlappedComponent :type Primitive%20Component%20Object%20Reference) (OtherActor :type Actor%20Object%20Reference) (OtherComp :type Primitive%20Component%20Object%20Reference) (OtherBodyIndex :type Integer) (bFromSweep :type Boolean) (SweepResult :type Hit%20Result%20Structure%20%28by%20ref%29))
  ;[1 1 1] Overlap with Aquilos Cap
  (bind _asbp_aquilos (Utilities|Casting|CastToBP_Aquilos OtherActor))
  (if (== (Variables|/Game/Aquilos/Blueprints/BP_Aquilos.BP_Aquilos_C|GetBox_Cap _asbp_aquilos) OtherComp)
    ;[1 1 1] Two Aquilos fixing knobs are unlocked
    (if (and (Utilities|Enum|Equal(Enum) (Variables|/Game/Aquilos/Blueprints/BP_Fixing_Knob.BP_Fixing_Knob_C|GetlockStatus (Variables|Knob|GetAquilosFixingKnobLeft)) "NewEnumerator1") (Utilities|Enum|Equal(Enum) (Variables|/Game/Aquilos/Blueprints/BP_Fixing_Knob.BP_Fixing_Knob_C|GetlockStatus (Variables|Knob|GetAquilosFixingKnobRight)) "NewEnumerator1"))
      ;[1 1 1] Attach to Aquilos
      (Transformation|AttachComponentToComponent (Variables|/Game/Aquilos/Blueprints/BP_Aquilos.BP_Aquilos_C|GetAquilos _asbp_aquilos) "S_Rod" "SnapToTarget" "SnapToTarget" "KeepWorld" true)
      (Variables|Default|SetisGrasp false)
      (Variables|Default|SetattachTo "NewEnumerator0"))))

(event EventBeginPlay
  (|CallParentFunction) ; This node is disabled and will not be called.\nDrag off pins to build functionality.
)

(event Collision|EventActorBeginOverlap
  (params (OtherActor :type Actor%20Object%20Reference))
  (|CallParentFunction OtherActor) ; This node is disabled and will not be called.\nDrag off pins to build functionality.
)

(event EventTick
  (params (DeltaSeconds :type Float%20%28single-precision%29))
  (|CallParentFunction DeltaSeconds)
  (Utilities|FlowControl|Sequence
    (:then_0
      (switch Utilities|FlowControl|Switch|SwitchonEnum_Rod_AttachTo (Variables|Default|GetattachTo)
        (:NewEnumerator0
          ;[1 1 1] Check knob lock status (if lock -> unpickable -> no collision)
          (if (or (Utilities|Enum|Equal(Enum) (Variables|/Game/Aquilos/Blueprints/BP_Fixing_Knob.BP_Fixing_Knob_C|GetlockStatus (Variables|Knob|GetAquilosFixingKnobLeft)) "NewEnumerator0") (Utilities|Enum|Equal(Enum) (Variables|/Game/Aquilos/Blueprints/BP_Fixing_Knob.BP_Fixing_Knob_C|GetlockStatus (Variables|Knob|GetAquilosFixingKnobRight)) "NewEnumerator0"))
            (Variables|Default|SetisPickable false)
            (Collision|SetActorEnableCollision false)
            (else
              (Variables|Default|SetisPickable true)
              (Collision|SetActorEnableCollision true))))
        (:NewEnumerator2
          (Variables|Default|SetisPickable true))))
    (:then_1
      (switch Utilities|FlowControl|Switch|SwitchonEnum_Rod_AttachTo (Variables|Default|GetattachTo)
        (:NewEnumerator0
          _)
        (:NewEnumerator1
          _))
      ;[1 1 1] If attached to hand, attach to <- else
      (Utilities|Casting|CastToBP_MotionController (Actor|GetAttachParentActor))
      (Variables|Default|SetattachTo "NewEnumerator2"))))

(event EventDisableCollisionCompoenents
  (Collision|SetCollisionEnabled (Variables|Default|GetBox_AttachToAquilos) "NoCollision"))

(event EventEnableCollisionComponenets
  (Collision|SetCollisionEnabled (Variables|Default|GetBox_AttachToAquilos) "QueryOnly"))

(fn ConstructionScript
  (|CallParentFunction))